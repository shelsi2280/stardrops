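; Star drop loot roller that upgrades a star tier on StarDrops input presses, then awards a gift.
; While iterations remain and the top tier is not reached, DropStar makes nested random rolls that can only raise the tier.
; Afterwards, a DoOnce draws a random gift from the GiftsTypes map entry for that tier.
; VisualStar and VisualGift only print the results as debug text.
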(event EventBeginPlay)

(event Collision|EventActorBeginOverlap
  (params (OtherActor :type Actor%20Object%20Reference)))

(event EventTick
  (params (DeltaSeconds :type Float%20%28single-precision%29)))

(event Input|ActionEvents|InputActionStarDrops
  (params (Key :type Key%20Structure :default "None"))
  (:Pressed
    (if (and (> (Variables|Default|GetIteration) 0) (Utilities|Enum|NotEqual(Enum) (Variables|Default|GetDropedStarType) "NewEnumerator3"))
      (bind (_star _startype) (CallFunction|DropStar))
      (Utilities|FlowControl|Sequence
        (:then_0
          (if (< (Math|Conversions|ToInteger(Byte) (Variables|Default|GetDropedStarType)) _star)
            (bind _output_get (Variables|Default|SetDropedStarType _startype))
            (CallFunction|VisualStar _output_get)))
        (:then_1
          (Math|Integer|DecrementInt (Variables|Default|GetIteration))))
      (else
        (Utilities|FlowControl|DoOnce false
          (:Completed
            (bind _gift (CallFunction|GetGift 0 (Variables|Default|GetDropedStarType)))
            (bind _output_get_2 (Variables|Default|SetDropedGift _gift))
            (CallFunction|VisualGift _output_get_2)))))))

(fn ConstructionScript)

(fn DropStar
  (Utilities|FlowControl|Sequence
    (:then_0
      (if (== (LocalVariables|GetL_Star) 0)
        (if (== (Math|Random|RandomIntegerinRange 0 5) 2)
          (LocalVariables|SetL_Star 1)
          (elif (== (Math|Random|RandomIntegerinRange 0 7) 2)
            (LocalVariables|SetL_Star 2)
            (elif (== (Math|Random|RandomIntegerinRange 0 10) 2)
              (LocalVariables|SetL_Star 3))))
        (elif (== (LocalVariables|GetL_Star) 1)
          (if (== (Math|Random|RandomIntegerinRange 0 5) 2)
            (LocalVariables|SetL_Star 2)
            (elif (== (Math|Random|RandomIntegerinRange 0 7) 2)
              (LocalVariables|SetL_Star 3)))
          (elif (== (LocalVariables|GetL_Star) 2)
            (if (== (Math|Random|RandomIntegerinRange 0 5) 0)
              (LocalVariables|SetL_Star 3))))))
    (:then_2
      (return (LocalVariables|GetL_Star) (Utilities|Select :Index (LocalVariables|GetL_Star) :Option%200 "NewEnumerator0" :Option%201 "NewEnumerator1" :Option%202 "NewEnumerator2" :Option%203 "NewEnumerator3")))))

(fn GetGift
  (params (Star :type Integer) (StarType :type E_Stars%20Enum :default "NewEnumerator0"))
  (bind _giftstypes (LocalVariables|GetGiftsTypes))
  (bind _value (Utilities|Map|Find _giftstypes StarType))
  (bind _gift (Utilities|Struct|BreakS_Gifts _value))
  (return (Utilities|Array|Get(acopy) _gift (Math|Random|RandomIntegerinRange 0 (- (Utilities|Array|Length _gift) 1)))))

(fn VisualStar
  (params (NewParam :type E_Stars%20Enum :default "NewEnumerator0"))
  ;[1 1 1] debug
  (Development|PrintString (Utilities|String|EnumtoString NewParam)))

(fn VisualGift
  (params (Enumerator :type E_gifts%20Enum :default "NewEnumerator0"))
  ;[1 1 1] Comment
  (Development|PrintString (Utilities|String|EnumtoString Enumerator) true true "(R=1.000000,G=0.595022,B=0.474500,A=1.000000)"))